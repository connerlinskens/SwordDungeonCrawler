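; Sword is a melee weapon actor that can be handed to a player and swung to create a timed hit window.
; Its Collider starts inactive on BeginPlay, and Attack activates it for a short delay before deactivating it again.
; GiveToPlayer sets the player as owner and attaches the sword to that actor, keeping relative transforms.
; The file itself contains no overlap or damage handling.
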(event `Attack`
  (`ActorComponent.SetActive` (`self.Collider`) true false)
  (`KismetSystemLibrary.Delay` 1.0)
  (`ActorComponent.SetActive` (`self.Collider`) false false))

(event `self.ReceiveBeginPlay`
  (`ActorComponent.SetActive` (`self.Collider`) false false))

(event `GiveToPlayer`
  (params (Player :type "PaperCharacter Object Reference"))
  (`self.SetOwner` Player)
  (`self.K2_AttachToActor` self Player "None" "KeepRelative" "KeepRelative" "KeepRelative" true))

(fn `UserConstructionScript`)